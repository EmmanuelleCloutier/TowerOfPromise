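; Checkpoint actor that records itself as the last checkpoint in the third-person GameMode when the player character overlaps its trigger.
; A timeline started on BeginPlay spins the static mesh in yaw while the checkpoint awaits activation.
; On activation it swaps the mesh to a copper material, turns off its point light and stops the spin as visual feedback.
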(event OnComponentBeginOverlap(Trigger)
  (params (OverlappedComponent :type Primitive%20Component%20Object%20Reference) (OtherActor :type Actor%20Object%20Reference) (OtherComp :type Primitive%20Component%20Object%20Reference) (OtherBodyIndex :type Integer) (bFromSweep :type Boolean) (SweepResult :type Hit%20Result%20Structure%20%28by%20ref%29))
  (bind _self self)
  (Utilities|Casting|CastToBP_ThirdPersonCharacter OtherActor)
  (bind _asbp_third_person_game_mode (Utilities|Casting|CastToBP_ThirdPersonGameMode (Game|GetGameMode)))
  (Variables|/Game/ThirdPerson/Blueprints/BP_ThirdPersonGameMode.BP_ThirdPersonGameMode_C|SetLastCheckpoint _asbp_third_person_game_mode _self)
  (Rendering|Material|SetMaterial (Variables|Default|GetStaticMesh _self) 0 "/Game/StarterContent/Materials/M_Metal_Copper.M_Metal_Copper")
  (Rendering|Components|Light|SetIntensity (Variables|Default|GetPointLight) 0.0)
  (CallFunction|StopRotation))

(event Custom|Stop%20Rotation
  (bind _rotation (Timeline|Movement Stop)
    (:Update
      (Transformation|SetRelativeRotation (Variables|Default|GetStaticMesh) (Math|Rotator|MakeRotator 0.0 0.0 _rotation) false false))))

(event EventBeginPlay
  (bind _rotation (Timeline|Movement Play)
    (:Update
      (Transformation|SetRelativeRotation (Variables|Default|GetStaticMesh) (Math|Rotator|MakeRotator 0.0 0.0 _rotation) false false))))

(fn ConstructionScript)