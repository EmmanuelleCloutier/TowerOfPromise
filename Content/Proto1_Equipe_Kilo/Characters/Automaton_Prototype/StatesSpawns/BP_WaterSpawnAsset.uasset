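; BP_WaterSpawnAsset is a temporary water puddle actor, apparently part of the Automaton prototype's liquid state.
; The puddle mesh starts hidden, then a DoOnce on Tick reveals it on the first tick.
; The ExpandPuddle timeline scales it from a flattened base size by PoolStretchFactor.
; When the timeline finishes, it calls IsWaitingTrue and LiquidEnd on the player's BP_ThirdPersonCharacter, then destroys itself.
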(event Custom|DoDahPuddleAnim
  (Rendering|SetVisibility (Variables|Default|GetWaterPuddle) true false)
  (bind _alpha (Timeline|ExpandPuddle PlayFromStart)
    (:Update
      (Transformation|SetRelativeScale3D (Variables|Default|GetWaterPuddle) (Math|Vector|Lerp(Vector) (Variables|Default|GetBase%20Scale) (* (Variables|Default|GetBase%20Scale) (Variables|Default|GetPool%20Stretch%20factor)) _alpha)))
    (:Finished
      (bind _asbp_third_person_character (Utilities|Casting|CastToBP_ThirdPersonCharacter (Game|GetPlayerCharacter 0)))
      (Default|IsWaitingTrue _asbp_third_person_character)
      (Default|LiquidEnd _asbp_third_person_character)
      (Actor|DestroyActor))))

(event EventBeginPlay
  (Variables|Default|SetBase%20Scale "0.100000,0.100000,0.250000")
  (Variables|Default|SetDefaultPuddleLocalTransform (Transformation|GetRelativeTransform (Variables|Default|GetWaterPuddle)))
  (Rendering|SetVisibility (Variables|Default|GetWaterPuddle) false false))

(event Collision|EventActorBeginOverlap
  (params (OtherActor :type Actor%20Object%20Reference)))

(event EventTick
  (params (DeltaSeconds :type Float%20%28single-precision%29))
  (Utilities|FlowControl|DoOnce false
    (:Completed
      (CallFunction|DoDahPuddleAnim))))

(fn ConstructionScript)