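; BP_PlatformSpawn is a short-lived platform spawn actor for the Automaton prototype that animates a cube growing into existence.
; On BeginPlay, a Timeline lerps the Cube's relative scale from zero toward PlatformScale.
; When the Timeline finishes, it calls IsWaitingTrue on player 0's BP_ThirdPersonCharacter, then destroys itself.
; If that character cast fails, the actor is not destroyed.
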(event EventBeginPlay
  (bind _alpha (Timeline|Timeline PlayFromStart)
    (:Update
      (Transformation|SetRelativeScale3D (Variables|Default|GetCube) (Math|Vector|Lerp(Vector) "0, 0, 0" (Variables|Default|GetPlatformScale) _alpha)))
    (:Finished
      (bind _asbp_third_person_character (Utilities|Casting|CastToBP_ThirdPersonCharacter (Game|GetPlayerCharacter 0)))
      (Default|IsWaitingTrue _asbp_third_person_character)
      (Actor|DestroyActor))))

(event Collision|EventActorBeginOverlap
  (params (OtherActor :type Actor%20Object%20Reference)))

(event EventTick
  (params (DeltaSeconds :type Float%20%28single-precision%29)))

(fn ConstructionScript)